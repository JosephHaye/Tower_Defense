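; Laser tower Blueprint that fires Bp_Laser actors at bp_Enemy actors within its Sphere1 overlap range.
; Overlap events maintain an enemy list, and the first entry starts a looping timer that spawns a laser at ShootingPoint aimed at the list's first enemy.
; An empty list resets the DoOnce, but the timer clear names "AttackEnemy1" instead of "AttackingEnemy1", so the timer keeps running idle.
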(event `self.Sphere1.OnComponentBeginOverlap`
  (params (OverlappedComponent :type "PrimitiveComponent Object Reference") (OtherActor :type "Actor Object Reference") (OtherComp :type "PrimitiveComponent Object Reference") (OtherBodyIndex :type Integer) (bFromSweep :type Boolean) (SweepResult :type "HitResult Structure (by ref)"))
  (bind _asbp_enemy (cast `/Game/EnemyAI/bp_Enemy` OtherActor))
  (`KismetArrayLibrary.Array_Add` (`self.ListOfEnemies`) _asbp_enemy)
  (`/Engine/EditorBlueprintResources/StandardMacros.DoOnce` false :!label _label
    (:`Completed`
      (`KismetSystemLibrary.K2_SetTimer` null "AttackingEnemy1" 0.5 true))))

(event `self.Sphere1.OnComponentEndOverlap`
  (params (OverlappedComponent :type "PrimitiveComponent Object Reference") (OtherActor :type "Actor Object Reference") (OtherComp :type "PrimitiveComponent Object Reference") (OtherBodyIndex :type Integer))
  (bind _asbp_enemy (cast `/Game/EnemyAI/bp_Enemy` OtherActor))
  (`KismetArrayLibrary.Array_RemoveItem` (`self.ListOfEnemies`) _asbp_enemy)
  (if (== (`KismetArrayLibrary.Array_Length` (`self.ListOfEnemies`)) 0)
    (`KismetSystemLibrary.K2_ClearTimer` null "AttackEnemy1")
    (goto _label :!via `Reset`)))

(fn `AttackingEnemy1`
  (bind _listofenemies (`self.ListOfEnemies`))
  (if (!= (`KismetArrayLibrary.Array_Length` _listofenemies) 0)
    (bind _returnvalue (`|SpawnActorFromClass` "/Game/Laser_Tower/bp_Laser.bp_Laser_C" (`SceneComponent.K2_GetComponentToWorld` (`self.ShootingPoint`)) "Undefined" "OverrideRootScale" null null))
    (set `/Game/Laser_Tower/bp_Laser.EnemyToAttack` (`|GetArrayItem` _listofenemies) _returnvalue)))

(fn `UserConstructionScript`)