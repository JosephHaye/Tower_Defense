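; Enemy character Blueprint that takes damage and dies when its health runs out.
; AnyDamage subtracts the incoming damage from Health and, at zero or below, destroys the actor through a DoOnce gate so death fires only once.
; The construction script applies the Speed variable to the movement component's max walk speed.
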(event `self.ReceiveAnyDamage`
  (params (Damage :type "Float (single-precision)") (DamageType :type "DamageType Object Reference") (InstigatedBy :type "Controller Object Reference") (DamageCauser :type "Actor Object Reference"))
  ;[1 1 1] Receive Damage
  (set `self.Health` (- (`self.Health`) Damage))
  (if (<= (`self.Health`) 0.0)
    (`/Engine/EditorBlueprintResources/StandardMacros.DoOnce` false
      (:`Completed`
        (`self.K2_DestroyActor`)))))

(fn `UserConstructionScript`
  (set `CharacterMovementComponent.MaxWalkSpeed` (`self.Speed`) (`self.CharacterMovement`)))