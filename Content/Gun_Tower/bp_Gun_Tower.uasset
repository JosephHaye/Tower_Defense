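; Gun tower Blueprint that tracks bp_Enemy actors inside its Range component and shoots Bp_Bullet from its Turret at one target.
; Range overlaps maintain an enemy list, and targeting picks the last entry when the current target is lost.
; Gated frame-delay loops, used instead of Tick, snap the turret onto the target or ease it back to rest when none remains.
; Once aimed, a ReFire timeline sized to FireDelay paces repeat shots.
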(event `Continous`
  ;[1 1 1] Fires at target
  (if (`self.CanShoot`)
    (if (== (`TimelineComponent.GetPlaybackPosition` (`self.ReFire`)) 0.0) :!label _label
      (`self.Fire`)
      (`Timeline|ReFire` :!label _label_2
        (:`Finished`
          (`self.ResetTimeline`)
          (`self.Continous`))))))

(event `StartFire`
  ;[1 1 1] Fires at target
  (`TimelineComponent.SetTimelineLength` (`self.ReFire`) (`self.FireDelay`))
  (goto _label))

(event `ResetTimeline`
  ;[1 1 1] Fires at target
  (`|ExecutionSequence`
    (:`then_0`
      (goto _label_2 :!via `Stop`))
    (:`then_1`
      (goto _label_2 :!via `SetNewTime`))))

(event `StopFire`
  ;[1 1 1] Fires at target
  (set `self.CanShoot` false)
  (`self.ResetFire`))

(event `Fire`
  ;[1 1 1] Fires at target
  (`/Engine/EditorBlueprintResources/StandardMacros.IsValid` (`self.Enemy`)
    (:`Is Valid`
      (`|SpawnActorFromClass` "/Game/Gun_Tower/bp_Bullet.bp_Bullet_C" (`KismetMathLibrary.MakeTransform` (.location (`SceneComponent.K2_GetComponentToWorld` (`self.Turret`))) (.rotation (`SceneComponent.K2_GetComponentToWorld` (`self.Turret`)))) "Undefined" "OverrideRootScale" null null))
    (:`Is Not Valid`
      (`self.StopFire`))))

(event `Target`
  (bind _listofenemies (`self.ListOfEnemies`))
  ;[1 1 1] Finds first target
  (if (`KismetArrayLibrary.Array_IsValidIndex` _listofenemies)
    (set `self.Enemy` (`|GetArrayItem` _listofenemies (`KismetArrayLibrary.Array_LastIndex` _listofenemies)))
    (`self.Aim`)
    (else
      (`self.Reset`))))

(event `Continue`
  (bind _enemy (`self.Enemy`))
  (bind _returnvalue (`KismetMathLibrary.MakeRotFromX` (`KismetMathLibrary.InverseTransformDirection` (`self.GetTransform`) (- (`self.Location`) (`SceneComponent.K2_GetComponentLocation` (`self.Turret`))))))
  ;[1 1 1] Aims
  (`/Engine/EditorBlueprintResources/StandardMacros.IsValid` (`self.Enemy`)
    (:`Is Valid`
      (`/Engine/EditorBlueprintResources/StandardMacros.Gate` true :!label _label_3
        (:`Exit`
          (`/Engine/EditorBlueprintResources/StandardMacros.IsValid` _enemy
            (:`Is Valid`
              (set `self.Location` (`self.K2_GetActorLocation` _enemy))
              (set `self.AimRotator` _returnvalue)
              (`SceneComponent.K2_SetRelativeRotation` (`self.Turret`) (`KismetMathLibrary.MakeRotator` 0.0 (.pitch _returnvalue) (.yaw _returnvalue)) false false)
              (if (== (`self.AimRotator`) (`KismetMathLibrary.MakeRotator` 0.0 (.pitch (`SceneComponent.RelativeRotation` (`self.Turret`))) (.yaw (`SceneComponent.RelativeRotation` (`self.Turret`)))) :`ErrorTolerance` 1.0)
                (`|ExecutionSequence`
                  (:`then_0`
                    (`/Engine/EditorBlueprintResources/StandardMacros.DoOnce` false :!label _label_4
                      (:`Completed`
                        (set `self.CanShoot` true)
                        (`self.StartFire`))))
                  (:`then_1`
                    (`KismetSystemLibrary.Delay` (`GameplayStatics.GetWorldDeltaSeconds`))
                    (`self.Continue`)))
                (else
                  (`self.StopFire`)
                  (`KismetSystemLibrary.Delay` (`GameplayStatics.GetWorldDeltaSeconds`))
                  (`self.Continue`))))
            (:`Is Not Valid`
              (`self.Cancel` :!label _label_5)
              (`self.Reset`)
              (`self.StopFire`))))))
    (:`Is Not Valid`
      (goto _label_5))))

(event `ResetFire`
  ;[1 1 1] Aims
  (goto _label_4 :!via `Reset`))

(event `Aim`
  ;[1 1 1] Aims
  (`|ExecutionSequence`
    (:`then_0`
      (goto _label_3 :!via `Open`))
    (:`then_1`
      (goto _label_3))))

(event `Cancel`
  ;[1 1 1] Aims
  (goto _label_3 :!via `Close`))

(event `ContinueReset`
  (bind _returnvalue (`KismetMathLibrary.RInterpTo_Constant` (`SceneComponent.RelativeRotation` (`self.Turret`)) (struct) (`GameplayStatics.GetWorldDeltaSeconds`) 50.0))
  ;[1 1 1] Resets
  (`/Engine/EditorBlueprintResources/StandardMacros.Gate` true :!label _label_6
    (:`Exit`
      (`/Engine/EditorBlueprintResources/StandardMacros.IsValid` (`self.Enemy`)
        (:`Is Valid`
          (`self.CancelReset` :!label _label_7))
        (:`Is Not Valid`
          (if (== _returnvalue (struct))
            (goto _label_7)
            (else
              (`SceneComponent.K2_SetRelativeRotation` (`self.Turret`) _returnvalue false false)
              (`KismetSystemLibrary.Delay` (`GameplayStatics.GetWorldDeltaSeconds`))
              (`self.ContinueReset`))))))))

(event `self.Range.OnComponentBeginOverlap`
  (params (OverlappedComponent :type "PrimitiveComponent Object Reference") (OtherActor :type "Actor Object Reference") (OtherComp :type "PrimitiveComponent Object Reference") (OtherBodyIndex :type Integer) (bFromSweep :type Boolean) (SweepResult :type "HitResult Structure (by ref)"))
  ;[1 1 1] Finds overlapping targets
  (bind _asbp_enemy (cast `/Game/EnemyAI/bp_Enemy` OtherActor))
  (`KismetArrayLibrary.Array_Add` (`self.ListOfEnemies`) _asbp_enemy)
  (`/Engine/EditorBlueprintResources/StandardMacros.IsValid` (`self.Enemy`)
    (:`Is Not Valid`
      (`self.Target`))))

(event `Reset`
  ;[1 1 1] Resets
  (`|ExecutionSequence`
    (:`then_0`
      (goto _label_6 :!via `Open`))
    (:`then_1`
      (goto _label_6))))

(event `CancelReset`
  ;[1 1 1] Resets
  (goto _label_6 :!via `Close`))

(event `self.Range.OnComponentEndOverlap`
  (params (OverlappedComponent :type "PrimitiveComponent Object Reference") (OtherActor :type "Actor Object Reference") (OtherComp :type "PrimitiveComponent Object Reference") (OtherBodyIndex :type Integer))
  (bind _listofenemies (`self.ListOfEnemies`))
  ;[1 1 1] Finds overlapping targets
  (bind _asbp_enemy (cast `/Game/EnemyAI/bp_Enemy` OtherActor))
  (if (`KismetArrayLibrary.Array_Contains` _listofenemies _asbp_enemy)
    (`KismetArrayLibrary.Array_RemoveItem` _listofenemies _asbp_enemy)
    (if (== _asbp_enemy (`self.Enemy`))
      (set `self.Enemy` null)
      (`self.Target`))))

(fn `UserConstructionScript`)