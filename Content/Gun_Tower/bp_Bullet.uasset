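; Tower bullet actor that damages enemies it overlaps and expires after travelling a set range.
; It records its spawn location on BeginPlay and destroys itself on Tick once its distance from that point reaches Range.
; Its sphere overlap applies Damage to the first bp_Enemy it touches, then destroys the bullet, with DoOnce guarding against repeat triggers.
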(event `self.ReceiveBeginPlay`
  (set `self.StartLocation` (`self.K2_GetActorLocation`)))

(event `self.ReceiveTick`
  (params (DeltaSeconds :type "Float (single-precision)"))
  (if (>= (`KismetMathLibrary.VSize` (- (`self.StartLocation`) (`self.K2_GetActorLocation`))) (`self.Range`))
    (`/Engine/EditorBlueprintResources/StandardMacros.DoOnce` false
      (:`Completed`
        (`self.K2_DestroyActor`)))))

(event `self.Sphere.OnComponentBeginOverlap`
  (params (OverlappedComponent :type "PrimitiveComponent Object Reference") (OtherActor :type "Actor Object Reference") (OtherComp :type "PrimitiveComponent Object Reference") (OtherBodyIndex :type Integer) (bFromSweep :type Boolean) (SweepResult :type "HitResult Structure (by ref)"))
  (bind _asbp_enemy (cast `/Game/EnemyAI/bp_Enemy` OtherActor))
  (`/Engine/EditorBlueprintResources/StandardMacros.DoOnce` false
    (:`Completed`
      (`GameplayStatics.ApplyDamage` _asbp_enemy (`self.Damage`) null self)
      (`self.K2_DestroyActor`))))

(fn `UserConstructionScript`)