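; Tower base actor that acts as a clickable tower area and opens the tower selection UI.
; Cursor events on the StaticMesh swap its material for hover, default, clicked and disabled states, with release always setting disabled.
; A click while TowerSpawned is true removes existing Bp_TowerSelector widgets, then creates a new one and passes itself as TowerArea.
; A click while it is false only shows the disabled material.
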(event `self.StaticMesh.OnBeginCursorOver`
  (params (TouchedComponent :type "PrimitiveComponent Object Reference"))
  (`PrimitiveComponent.SetMaterial` (`self.StaticMesh`) 0 "/Game/Materials/Mouse_Over.Mouse_Over"))

(event `self.StaticMesh.OnEndCursorOver`
  (params (TouchedComponent :type "PrimitiveComponent Object Reference"))
  (`PrimitiveComponent.SetMaterial` (`self.StaticMesh`) 0 "/Game/Materials/Default.Default"))

(event `self.StaticMesh.OnClicked`
  (params (TouchedComponent :type "PrimitiveComponent Object Reference") (ButtonPressed :type "Key Structure"))
  (bind _staticmesh (`self.StaticMesh`))
  (if (`self.TowerSpawned`)
    (`PrimitiveComponent.SetMaterial` _staticmesh 0 "/Game/Materials/Clicked.Clicked")
    (bind _foundwidgets (`WidgetBlueprintLibrary.GetAllWidgetsOfClass` "/Game/bp_TowerSelector.bp_TowerSelector_C" false))
    (for _array_element _foundwidgets
      (`Widget.RemoveFromParent` _array_element))
    (bind _returnvalue (`|GenericCreateObject` "/Game/bp_TowerSelector.bp_TowerSelector_C" self))
    (`UserWidget.AddToViewport` _returnvalue 0)
    (set `/Game/bp_TowerSelector.TowerArea` self _returnvalue)
    (else
      (`PrimitiveComponent.SetMaterial` _staticmesh 0 "/Game/Materials/Disabled.Disabled"))))

(event `self.StaticMesh.OnReleased`
  (params (TouchedComponent :type "PrimitiveComponent Object Reference") (ButtonReleased :type "Key Structure"))
  (`PrimitiveComponent.SetMaterial` (`self.StaticMesh`) 0 "/Game/Materials/Disabled.Disabled"))

(fn `UserConstructionScript`)